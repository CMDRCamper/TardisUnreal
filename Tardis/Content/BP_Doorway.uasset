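; BP_Doorway is a doorway actor that shows the view from a BP_biggerCam scene capture on its mesh, apparently for a TARDIS-style portal effect.
; The construction script creates a dynamic material on the doorway mesh, and BeginPlay caches the first BP_biggerCam found in the level.
; Every Tick assigns that camera's render target to the material's "Screen Texture" parameter and prints the texture's name for debugging.
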(event `self.ReceiveBeginPlay`
  (bind _outactors (`GameplayStatics.GetAllActorsOfClass` "/Game/BP_biggerCam.BP_biggerCam_C"))
  (set `self.tardisCam` (`|GetArrayItem` _outactors)))

(event `self.ReceiveTick`
  (params (DeltaSeconds :type "Float (single-precision)"))
  (bind _doorwaymat (`self.doorwayMat`))
  (`MaterialInstanceDynamic.SetTextureParameterValue` _doorwaymat "Screen Texture" (`SceneCaptureComponent2D.TextureTarget` (`/Game/BP_biggerCam.SceneCaptureComponent2D` (`self.tardisCam`))))
  (bind _returnvalue (`MaterialInstanceDynamic.K2_GetTextureParameterValue` _doorwaymat "Screen Texture"))
  (`KismetSystemLibrary.PrintString` (`KismetSystemLibrary.GetDisplayName` _returnvalue)))

(fn `UserConstructionScript`
  (bind _returnvalue (`PrimitiveComponent.CreateDynamicMaterialInstance` (`self.DoorwayMesh`) 0 null "None"))
  (set `self.doorwayMat` _returnvalue))