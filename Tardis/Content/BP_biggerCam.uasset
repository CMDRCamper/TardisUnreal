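; Scene capture camera that renders a view to textures, adjusted each tick by the player's position relative to the BP_Doorway actor for a parallax effect.
; It yaws by the player's angle around the doorway, offset by the doorway's rotation.
; FOV narrows with squared distance between MaxFov and MinFov, with a fixed fallback below that range.
; Distance thresholds swap among four render targets as LODs; the camera dolly nodes never run.
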(event `self.ReceiveBeginPlay`
  (bind _returnvalue (`GameplayStatics.GetActorOfClass` "/Game/FirstPerson/Blueprints/BP_FirstPersonCharacter.BP_FirstPersonCharacter_C"))
  (set `self.Player` _returnvalue)
  (bind _returnvalue_2 (`GameplayStatics.GetActorOfClass` "/Game/BP_Doorway.BP_Doorway_C"))
  (set `self.doorWay` _returnvalue_2))

(event `self.ReceiveTick`
  (params (DeltaSeconds :type "Float (single-precision)"))
  (`self.cameraParallax`)
  (`self.scaleFOV`)
  (`self.scaleCaptureTexture`))

(fn `cameraParallax`
  (bind (_x _y) (`KismetMathLibrary.BreakVector3f` (.location (`self.GetTransform` (`self.Player`)))))
  (bind (_x_2 _y_2) (`KismetMathLibrary.BreakVector3f` (.location (`self.GetTransform` (`self.doorWay`)))))
  (bind _output_get (set `self.Xdistance` (- _x _x_2)))
  (bind _output_get_2 (set `self.Ydistance` (- _y_2 _y)))
  (`self.K2_SetActorRotation` (`KismetMathLibrary.MakeRotator` (.roll (`self.K2_GetActorRotation` self)) (.pitch (`self.K2_GetActorRotation` self)) (- (`KismetMathLibrary.DegAtan2` _output_get _output_get_2) (.yaw (`SceneComponent.RelativeRotation` (`/Game/BP_Doorway.DefaultSceneRoot` (`self.doorWay`))))))))

(fn `scaleCaptureTexture`
  (locals (distance :type "Float (double-precision)"))
  (bind _scenecapturecomponent2d (`self.SceneCaptureComponent2D`))
  (bind _output_get (set `local.distance` (`KismetMathLibrary.Sqrt` (+ (`KismetMathLibrary.Square` (`self.Ydistance`)) (`KismetMathLibrary.Square` (`self.Xdistance`))))))
  (if (>= _output_get 2000.0)
    (set `SceneCaptureComponent2D.TextureTarget` (`self.superLowText`) _scenecapturecomponent2d)
    (elif (>= _output_get 1000.0)
      (set `SceneCaptureComponent2D.TextureTarget` (`self.ldText`) _scenecapturecomponent2d)
      (elif (>= _output_get 500.0)
        (set `SceneCaptureComponent2D.TextureTarget` (`self.mdText`) _scenecapturecomponent2d)
        (else
          (set `SceneCaptureComponent2D.TextureTarget` (`self.hdText`) _scenecapturecomponent2d))))))

(fn `scaleFOV`
  (locals (distance :type "Float (double-precision)"))
  (bind _maxfov (`self.maxFov`))
  (bind _scenecapturecomponent2d (`self.SceneCaptureComponent2D`))
  (bind _returnvalue (<= (`local.distance`) 2000.0))
  ;[1 1 1] Scale FOV up or down until it reaches a certain point as the player gets closer or further from the doorway
  (bind _output_get (set `local.distance` (`KismetMathLibrary.Sqrt` (+ (`KismetMathLibrary.Square` (`self.Ydistance`)) (`KismetMathLibrary.Square` (`self.Xdistance`))))))
  (bind _returnvalue_2 (/ (`self.maxFov`) (+ (* (* (`KismetMathLibrary.Square` _output_get) 0.0001) 0.001) 1.0)))
  (if (< _returnvalue_2 _maxfov)
    (if (> _returnvalue_2 (`self.minFov`))
      (set `SceneCaptureComponent2D.FOVAngle` _returnvalue_2 _scenecapturecomponent2d)
      ;[1 1 1] Move camera further away or closer depending on distance
      (if (< (`local.distance`) (`self.prevDistance`))
        (if (not _returnvalue)
          (set `self.prevDistance` (`local.distance`) :!label _label))
        (elif _returnvalue
          (if (not (> (`local.distance`) (`self.prevDistance`)))
            (goto _label))
          (else
            (goto _label))))
      (else
        (set `SceneCaptureComponent2D.FOVAngle` 60.0 _scenecapturecomponent2d)))
    (else
      (set `SceneCaptureComponent2D.FOVAngle` _maxfov _scenecapturecomponent2d))))

(fn `UserConstructionScript`)